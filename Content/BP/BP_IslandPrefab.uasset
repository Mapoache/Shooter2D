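; BP_IslandPrefab is an island actor with random scale and tilt that animates continuously through orbit-style rotation.
; The construction script sets two spring arm lengths from variables; BeginPlay picks one of two scale ranges via NearFar and randomly rotates the Island component.
; A self-restarting Orbit timeline adds constant, differing rotation increments to both arms each update.
; The arms' rotations are saved at start and after each cycle but never read here.
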(event `self.ReceiveBeginPlay`
  (bind _returnvalue (`KismetMathLibrary.RandomFloatInRange` 5.0 20.0))
  (bind _returnvalue_2 (`KismetMathLibrary.RandomFloatInRange` 1.0 10.0))
  (set `self.Spring01LastRotation` (`SceneComponent.K2_GetComponentRotation` (`self.SpringArm01`)))
  (set `self.Spring02LastRotation` (`SceneComponent.K2_GetComponentRotation` (`self.SpringArm02`)))
  (if (`self.Near/Far?`)
    ;[1 1 1] Set Random Scale
    (`self.SetActorScale3D` (`KismetMathLibrary.MakeVector` _returnvalue_2 _returnvalue_2 _returnvalue_2))
    (else
      (`self.SetActorScale3D` (`KismetMathLibrary.MakeVector` _returnvalue _returnvalue _returnvalue))))
  ;[1 1 1] Set Random Initial Rotation
  (`SceneComponent.K2_AddRelativeRotation` (`self.Island`) (`KismetMathLibrary.MakeRotator` (`KismetMathLibrary.RandomFloatInRange` -35.0 35.0) (`KismetMathLibrary.RandomFloatInRange` -35.0 35.0) (`KismetMathLibrary.RandomFloatInRange` -35.0 35.0)) false false)
  (`self.StartOrbit`))

(event `StartOrbit`
  ;[1 1 1] Orbit
  (`Timeline|Orbit`
    (:`Update`
      (`SceneComponent.K2_AddWorldRotation` (`self.SpringArm01`) (`KismetMathLibrary.MakeRotator` 0.1 -0.1) false false)
      (`SceneComponent.K2_AddWorldRotation` (`self.SpringArm02`) (`KismetMathLibrary.MakeRotator` -0.1 0.04) false false))
    (:`Finished`
      (switch `ETimelineDirection` "Forward"
        (:`Forward`
          (set `self.Spring01LastRotation` (`SceneComponent.K2_GetComponentRotation` (`self.SpringArm01`)))
          (set `self.Spring02LastRotation` (`SceneComponent.K2_GetComponentRotation` (`self.SpringArm02`)))
          (`self.StartOrbit`))))))

(fn `UserConstructionScript`
  (set `SpringArmComponent.TargetArmLength` (`self.CustomArmLenght01`) (`self.SpringArm01`))
  (set `SpringArmComponent.TargetArmLength` (`self.CustomArmLength02`) (`self.SpringArm02`)))