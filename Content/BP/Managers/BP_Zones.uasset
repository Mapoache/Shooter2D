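; BP_Zones is a trigger zone that activates spawners when the player's spaceship enters it.
; The first SpaceShipPawn overlap with its Box calls Init on the first two entries of the Spawners array and prints a debug message, gated by a DoOnce that is never reset.
; Any actor leaving the Box sets Stop to false on both spawners, with no cast check.
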(event `self.Box.OnComponentBeginOverlap`
  (params (OverlappedComponent :type "PrimitiveComponent Object Reference") (OtherActor :type "Actor Object Reference") (OtherComp :type "PrimitiveComponent Object Reference") (OtherBodyIndex :type Integer) (bFromSweep :type Boolean) (SweepResult :type "HitResult Structure (by ref)"))
  (cast `SpaceShipPawn` OtherActor)
  (`/Engine/EditorBlueprintResources/StandardMacros.DoOnce` false
    (:`Completed`
      (`/Game/BP/Managers/BP_EnemySpawner.Init` (`|GetArrayItem` (`self.Spawners`)))
      (`/Game/BP/Managers/BP_EnemySpawner.Init` (`|GetArrayItem` (`self.Spawners`) 1))
      (`KismetSystemLibrary.PrintString` "ZONA ACTIVADA"))))

(event `self.Box.OnComponentEndOverlap`
  (params (OverlappedComponent :type "PrimitiveComponent Object Reference") (OtherActor :type "Actor Object Reference") (OtherComp :type "PrimitiveComponent Object Reference") (OtherBodyIndex :type Integer))
  (bind _spawners (`self.Spawners`))
  (set `/Game/BP/Managers/BP_EnemySpawner.Stop?` false (`|GetArrayItem` _spawners 1))
  (set `/Game/BP/Managers/BP_EnemySpawner.Stop?` false (`|GetArrayItem` _spawners)))

(fn `UserConstructionScript`)