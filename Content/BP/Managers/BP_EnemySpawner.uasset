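; Enemy spawner actor that periodically spawns BP_EnemyPawn at its own transform, armed with BP_EnemyBullet projectiles.
; Init runs on BeginPlay when StartInit is set and starts a looping timer, its random interval rolled once.
; Each tick of the timer skips spawning if Stop is set or the world-wide enemy count exceeds its limit.
; A per-spawner counter caps total spawns at five, though the timer keeps looping afterwards.
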(event `self.ReceiveBeginPlay`
  (if (`self.StartInit?`)
    (`self.Init`)))

(event `Init`
  (`KismetSystemLibrary.K2_SetTimerDelegate` (delegate `StartWaves`) (`KismetMathLibrary.RandomFloatInRange` 5.0 8.0) true))

(event `StartWaves`
  (bind _spawncount (`self.SpawnCount`))
  (if (not (`self.Stop?`))
    (bind _newparam (`self.CheckMaximumEnemies`))
    (if (not _newparam)
      (`/Engine/EditorBlueprintResources/StandardMacros.IncrementInt` _spawncount
        (:`  `
          (if (not (> _spawncount 5))
            (`|SpawnActorFromClass` "/Game/BP/Pawns/BP_EnemyPawn.BP_EnemyPawn_C" (`self.GetTransform`) "AlwaysSpawn" "MultiplyWithRoot" null "/Game/BP/Bullets/BP_EnemyBullet.BP_EnemyBullet_C" null)))))))

(fn `CheckMaximumEnemies`
  (returns (NewParam :type Boolean))
  (bind _outactors (`GameplayStatics.GetAllActorsOfClass` "/Game/BP/Pawns/BP_EnemyPawn.BP_EnemyPawn_C"))
  (return (> (`KismetArrayLibrary.Array_Length` _outactors) 8)))

(fn `UserConstructionScript`)