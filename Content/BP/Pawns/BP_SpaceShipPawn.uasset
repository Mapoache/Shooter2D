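; Player spaceship pawn for a 2D shooter that aims at the mouse, fires single or power-up triple-spread bullets, and opens a pause menu.
; It creates the HUD, updates health and height values each tick, and drives a timeline-based fire cooldown.
; Damage passes to a HealthComponent with brief invincibility.
; Death or victory saves loss/win counts through GI_2DShooter, then fades and reloads the level; victory also clears spawners and enemies.
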(event `self.ReceiveBeginPlay`
  ;[1 1 1] Init
  (bind _returnvalue (`|CreateWidget` "/Game/BP/WG/WG_PlayerHUD.WG_PlayerHUD_C"))
  (bind _output_get (set `self.HUD` _returnvalue))
  (`UserWidget.AddToViewport` _output_get 0)
  (bind _asgi_2dshooter (cast `/Game/BP/Managers/GI_2DShooter` (`GameplayStatics.GetGameInstance`)))
  (`/Game/BP/Managers/GI_2DShooter.LoadGameData` _asgi_2dshooter)
  (set `self.Wins` (`/Game/BP/Managers/GI_2DShooter.CurrentWins` _asgi_2dshooter))
  (set `self.Loses` (`/Game/BP/Managers/GI_2DShooter.CurrentLoses` _asgi_2dshooter))
  (`SceneComponent.K2_AttachToComponent` (`self.SpringArmComponent`) (`self.CapsuleComponent`) "None" "KeepRelative" "KeepRelative" "KeepRelative" true))

(event `CheckXAxis`
  ;[1 1 1] Check X Axis
  (if (!= (.y (`self.K2_GetActorLocation`)) 0.0)
    _))

(event `self.ReceiveTick`
  (params (DeltaSeconds :type "Float (single-precision)"))
  ;[1 1 1] Ship Rotation
  (if (not (`self.Dead?`))
    (`SceneComponent.K2_SetWorldRotation` (`self.CapsuleComponent`) (`self.Get Rotation from Mouse Direction`) false false)
    (`self.SetWidgetVariables`)))

(event `self.OnFirePressed`
  (params (AimDirection :type "Vector Structure"))
  (bind _arrow (`self.Arrow`))
  ;[1 1 1] Fire
  (`GameplayStatics.PlaySound2D` "/Game/Sounds/Shoot.Shoot" 1.0 1.0 0.0 null null)
  (if (`self.PowerUp?`)
    (`self.TripleShoot`)
    (else
      (`|SpawnActorFromClass` "/Game/BP/Bullets/BP_Bullet.BP_Bullet_C" (`KismetMathLibrary.MakeTransform` (`SceneComponent.K2_GetComponentLocation` _arrow) (`SceneComponent.K2_GetComponentRotation` _arrow)) "AlwaysSpawn" "MultiplyWithRoot" null null)))
  (`/Game/BP/WG/WG_PlayerHUD.Event Cooldown` (`self.HUD`))
  (bind (_direction _cooldown) (`Timeline|CooldownAnim` :!via `PlayFromStart`)
    (:`Update`
      (set `self.Cooldown` _cooldown))))

(event `SetPowerUp`
  (bind _hud (`self.HUD`))
  (`UserWidget.PlayAnimation` _hud (`/Game/BP/WG/WG_PlayerHUD.LevelUp` _hud) 0.0 1 "Forward" 1.0 false)
  (set `self.PowerUp?` true))

(event `/Game/BP/Managers/BPI_Damager.ReceiveDamage`
  (params (DamageIn :type "Float (double-precision)"))
  ;[1 1 1] Damage Event
  (if (not (`self.Invincible?`))
    (`HealthComponent.TakeDamage` (`self.HealthComponent`) DamageIn)
    (set `self.Invincible?` true)
    (`KismetSystemLibrary.Delay` (`self.InvincibilityDuration`))
    (set `self.Invincible?` false)))

(event `self.HealthComponent.OnPawnDied`
  ;[1 1 1] Handle Death
  (`/Engine/EditorBlueprintResources/StandardMacros.DoOnce` false
    (:`Completed`
      (`self.DisableInput` (`GameplayStatics.GetPlayerController` 0))
      (bind _asgi_2dshooter (cast `/Game/BP/Managers/GI_2DShooter` (`GameplayStatics.GetGameInstance`)))
      (`/Engine/EditorBlueprintResources/StandardMacros.IncrementInt` (`/Game/BP/Managers/GI_2DShooter.CurrentLoses` _asgi_2dshooter)
        (:`  `
          (`/Game/BP/Managers/GI_2DShooter.SaveGameData` _asgi_2dshooter)
          (`/Game/BP/WG/WG_PlayerHUD.FadeIn` (`self.HUD`))
          (`KismetSystemLibrary.Delay` 2.0)
          (`GameplayStatics.OpenLevel` "SpaceShipLevel01"))))))

(event `Event Win`
  ;[1 1 1] Win Event
  (`self.DisableInput` (`GameplayStatics.GetPlayerController` 0))
  (`GameplayStatics.PlaySound2D` "/Game/Sounds/SFX_Win.SFX_Win" 1.0 1.0 0.0 null null)
  (bind _outactors (`GameplayStatics.GetAllActorsOfClass` "/Game/BP/Managers/BP_EnemySpawner.BP_EnemySpawner_C"))
  (for _array_element _outactors
    (set `/Game/BP/Managers/BP_EnemySpawner.Stop?` true _array_element)
    (`self.K2_DestroyActor` _array_element))
  (bind _outactors_2 (`GameplayStatics.GetAllActorsOfClass` "/Game/BP/Pawns/BP_EnemyPawn.BP_EnemyPawn_C"))
  (for _array_element_2 _outactors_2
    (`/Game/BP/Pawns/BP_EnemyPawn.Custom Death` _array_element_2))
  (bind _asgi_2dshooter (cast `/Game/BP/Managers/GI_2DShooter` (`GameplayStatics.GetGameInstance`)))
  (`/Engine/EditorBlueprintResources/StandardMacros.IncrementInt` (`/Game/BP/Managers/GI_2DShooter.CurrentWins` _asgi_2dshooter)
    (:`  `
      (`/Game/BP/Managers/GI_2DShooter.SaveGameData` _asgi_2dshooter)
      (`/Game/BP/WG/WG_PlayerHUD.FadeIn` (`self.HUD`))
      (`KismetSystemLibrary.Delay` 2.0)
      (`GameplayStatics.OpenLevel` "SpaceShipLevel01"))))

(event `Event BacktoX0`
  (bind _returnvalue (`self.K2_GetActorLocation`))
  ;[1 1 1] Fix Location when Collide
  (bind (_direction _newtrack_0) (`Timeline|BackToX0`)
    (:`Update`
      (`self.K2_SetActorLocation` (`KismetMathLibrary.VLerp` _returnvalue (`KismetMathLibrary.MakeVector` (.x _returnvalue) 0.0 (.z _returnvalue)) _newtrack_0) true))))

(event `Key|One`
  (params (Key :type "Key Structure"))
  (:`Pressed`
    (`GameplayStatics.SetGlobalTimeDilation` 0.0 :!label _label)
    (bind _returnvalue (`|CreateWidget` "/Game/BP/WG/WG_PauseMenu.WG_PauseMenu_C"))
    (set `UserWidget.Priority` 1 _returnvalue)
    (`UserWidget.AddToViewport` _returnvalue 0)
    (set `PlayerController.bShowMouseCursor` true (`GameplayStatics.GetPlayerController` 0))))

(event `Key|Escape`
  (params (Key :type "Key Structure"))
  (:`Pressed`
    (goto _label)))

(fn `SetWidgetVariables`
  (bind (_returnvalue_x _returnvalue_y _returnvalue_z) (`KismetMathLibrary.BreakVector` (`self.K2_GetActorLocation`)))
  (bind _healthcomponent (`self.HealthComponent`))
  (set `self.WorldHeight` _returnvalue_z)
  (set `self.CurrentHealthNormalized` (/ (`HealthComponent.CurrentHealth` _healthcomponent) (`HealthComponent.MaxHealth` _healthcomponent))))

(fn `TripleShoot`
  (bind _arrow (`self.Arrow`))
  (bind _returnvalue (`SceneComponent.K2_GetComponentRotation` _arrow))
  (for _index (range 3)
    (`|SpawnActorFromClass` "/Game/BP/Bullets/BP_Bullet.BP_Bullet_C" (`KismetMathLibrary.MakeTransform` (`SceneComponent.K2_GetComponentLocation` _arrow) (select `int` _index :`0` (`KismetMathLibrary.MakeRotator` (.roll _returnvalue) (+ (.pitch _returnvalue) 25.0) (.yaw _returnvalue)) :`1` _returnvalue :`2` (`KismetMathLibrary.MakeRotator` (.roll _returnvalue) (- (.pitch _returnvalue) 25.0) (.yaw _returnvalue)))) "AdjustIfPossibleButAlwaysSpawn" "MultiplyWithRoot" null null)))

(fn `UserConstructionScript`)