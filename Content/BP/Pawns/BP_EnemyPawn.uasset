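; Enemy pawn that damages the player's spaceship on capsule overlap and shows a floating health bar.
; Damage goes to a HealthComponent and plays an explosion sound, while the bar drops by a fixed step independent of the damage amount.
; Each tick the health widget yaws toward the player's camera.
; HealthComponent death destroys the pawn immediately; a separate CustomDeath event adds a Niagara explosion and delayed destruction.
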(event `self.ReceiveBeginPlay`
  (`parent.ReceiveBeginPlay`)
  (`self.SetInitialVariablesAndReferences`))

(event `self.ReceiveTick`
  (params (DeltaSeconds :type "Float (single-precision)"))
  (`parent.ReceiveTick` DeltaSeconds)
  (`self.RotateHealthBar`))

(event `self.CapsuleComponent.OnComponentBeginOverlap`
  (params (OverlappedComponent :type "PrimitiveComponent Object Reference") (OtherActor :type "Actor Object Reference") (OtherComp :type "PrimitiveComponent Object Reference") (OtherBodyIndex :type Integer) (bFromSweep :type Boolean) (SweepResult :type "HitResult Structure (by ref)"))
  (bind _asbp_space_ship_pawn (cast `/Game/BP/Pawns/BP_SpaceShipPawn` OtherActor))
  (`/Game/BP/Pawns/BP_SpaceShipPawn.ReceiveDamage` _asbp_space_ship_pawn 25.0))

(event `/Game/BP/Managers/BPI_Damager.ReceiveDamage`
  (params (DamageIn :type "Float (double-precision)"))
  (`HealthComponent.TakeDamage` (`self.HealthComponent`) DamageIn)
  (`GameplayStatics.PlaySound2D` "/Game/StarterContent/Audio/Explosion01.Explosion01" 1.0 1.0 0.0 null null)
  (bind _output_get (set `self.HealthFloat` (- (`self.HealthFloat`) 0.35)))
  (`ProgressBar.SetPercent` (`self.HealthBar`) _output_get))

(event `Custom Death`
  (bind _widget (`self.Widget`))
  (`NiagaraFunctionLibrary.SpawnSystemAtLocation` "/Game/VFX/NS_SimpleExplosion.NS_SimpleExplosion" (`SceneComponent.K2_GetComponentLocation` _widget) (`SceneComponent.K2_GetComponentRotation` _widget))
  (`KismetSystemLibrary.Delay` 1.0)
  (`self.K2_DestroyActor`))

(event `self.HealthComponent.OnPawnDied`
  (`self.K2_DestroyActor`))

(fn `RotateHealthBar`
  (`SceneComponent.K2_SetWorldRotation` (`self.Widget`) (`KismetMathLibrary.MakeRotator` 0.0 0.0 (.yaw (`KismetMathLibrary.FindLookAtRotation` (`SceneComponent.K2_GetComponentLocation` (`self.Widget`)) (`SceneComponent.K2_GetComponentLocation` (`SpaceShipPawn.CameraComponent` (`self.PawnRef`)))))) false false))

(fn `SetInitialVariablesAndReferences`
  (bind _aswg_enemy_life (cast `/Game/BP/WG/WG_EnemyLife` (`WidgetComponent.GetUserWidgetObject` (`self.Widget`))))
  (bind _output_get (set `self.HealthBar` (`/Game/BP/WG/WG_EnemyLife.ProgressBar_74` _aswg_enemy_life)))
  (`ProgressBar.SetPercent` _output_get 1.0)
  (bind _asbp_space_ship_pawn (cast `/Game/BP/Pawns/BP_SpaceShipPawn` (`GameplayStatics.GetPlayerPawn` 0))
    (:`then`
      (set `self.PawnRef` _asbp_space_ship_pawn))
    (:`CastFailed`
      (`KismetSystemLibrary.PrintString` "BADPLAYER"))))

(fn `UserConstructionScript`)