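; Enemy projectile actor that damages the player when its collision component overlaps them.
; On overlap with an actor tagged Player, a DoOnce gate spawns a half-scale Niagara explosion at the impact point, oriented to the impact normal.
; If that actor implements BPI_Damager, it receives a fixed damage message and the bullet destroys itself.
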(event `self.CollisionComponent.OnComponentBeginOverlap`
  (params (OverlappedComponent :type "PrimitiveComponent Object Reference") (OtherActor :type "Actor Object Reference") (OtherComp :type "PrimitiveComponent Object Reference") (OtherBodyIndex :type Integer) (bFromSweep :type Boolean) (SweepResult :type "HitResult Structure (by ref)"))
  (bind (_bblockinghit _binitialoverlap _time _distance _location _impactpoint _normal _impactnormal) (`GameplayStatics.BreakHitResult` SweepResult))
  (`/Engine/EditorBlueprintResources/StandardMacros.IsValid` OtherActor
    (:`Is Valid`
      (if (`self.ActorHasTag` OtherActor "Player")
        (`/Engine/EditorBlueprintResources/StandardMacros.DoOnce` false
          (:`Completed`
            (`NiagaraFunctionLibrary.SpawnSystemAtLocation` "/Game/VFX/NS_SimpleExplosion.NS_SimpleExplosion" _impactpoint (`KismetMathLibrary.MakeRotFromZ` _impactnormal) (0.5 0.5 0.5))
            (if (`KismetSystemLibrary.DoesImplementInterface` OtherActor "/Game/BP/Managers/BPI_Damager.BPI_Damager_C")
              (message `/Game/BP/Managers/BPI_Damager.ReceiveDamage` OtherActor 25.0)
              (`self.K2_DestroyActor`))))))))

(fn `UserConstructionScript`)